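; Melee punch weapon for Drake that extends a parent weapon's Check Hit to deal damage around whatever the fist strikes.
; Check Hit calls the parent, then runs a stationary multi sphere trace at the Sphere component against WorldDynamic objects, ignoring the owning Character.
; Each hit feeds DamageRadial with the Damage value and a small radius.
; The trace radius comes from the sphere's shape scale rather than its radius, and debug drawing is on.
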(event EventBeginPlay
  (|CallParentFunction) ; This node is disabled and will not be called.\nDrag off pins to build functionality.
)

(event Collision|EventActorBeginOverlap
  (params (OtherActor :type Actor%20Object%20Reference))
  (|CallParentFunction OtherActor) ; This node is disabled and will not be called.\nDrag off pins to build functionality.
)

(event EventTick
  (params (DeltaSeconds :type Float%20%28single-precision%29))
  (|CallParentFunction DeltaSeconds) ; This node is disabled and will not be called.\nDrag off pins to build functionality.
)

(fn ConstructionScript
  (|CallParentFunction))

(fn CheckHit
  (bind _sphere (Variables|Default|GetSphere))
  (bind _returnvalue (Transformation|GetSocketLocation _sphere "None"))
  (|CallParentFunction)
  (bind _outhits (Collision|MultiSphereTraceForObjects _returnvalue _returnvalue (Class|SphereComponent|GetShapeScale (Variables|Default|GetSphere)) (Utilities|Array|MakeArray "ObjectTypeQuery2") false (Utilities|Array|MakeArray (Variables|Default|GetCharacter)) "ForOneFrame"))
  (for _array_element _outhits
    (CallFunction|DamageRadial _array_element (Variables|Default|GetDamage) 5.0 self)))