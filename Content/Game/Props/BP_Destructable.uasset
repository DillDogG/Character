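; BP_Destructable is a destructible prop with a configurable static mesh, set in the construction script, and optional physics simulation.
; RadialDamage passes through a DoOnce with no reset shown, then subtracts the damage from Health.
; At zero Health or below, the actor is destroyed with an explosion emitter at the mesh location.
; Otherwise it plays a hit sound, and a Simulate branch and trailing delay lead to no further action.
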(event EventBeginPlay
  (Physics|SetSimulatePhysics (Variables|Default|GetStaticMesh) (Variables|Default|GetSimulate)))

(event Collision|EventActorBeginOverlap
  (params (OtherActor :type Actor%20Object%20Reference)))

(event EventTick
  (params (DeltaSeconds :type Float%20%28single-precision%29)))

(event Game|Damage|EventRadialDamage
  (params (DamageReceived :type Float%20%28single-precision%29) (DamageType :type Damage%20Type%20Object%20Reference) (Origin :type Vector :default "0, 0, 0") (HitInfo :type Hit%20Result%20Structure%20%28by%20ref%29) (InstigatedBy :type Controller%20Object%20Reference) (DamageCauser :type Actor%20Object%20Reference))
  (Utilities|FlowControl|DoOnce false
    (:Completed
      (bind _output_get (Variables|Default|SetHealth (- (Variables|Default|GetHealth) DamageReceived)))
      (if (<= _output_get 0.0)
        (Actor|DestroyActor)
        (Effects|SpawnEmitteratLocation "/Game/StarterContent/Particles/P_Explosion.P_Explosion" (Transformation|GetWorldLocation (Variables|Default|GetStaticMesh)))
        (else
          (Audio|PlaySound2D "/Game/Game/hit_fx.hit_fx" 1.0 1.0 0.0 0 0)
          (if (Variables|Default|GetSimulate)
            _
            (else
              _))
          (Utilities|FlowControl|Delay 2.0))))))

(fn ConstructionScript
  (bind _mesh (Variables|Default|GetMesh))
  (Utilities|IsValid _mesh
    (:Is%20Valid
      (Components|StaticMesh|SetStaticMesh (Variables|Default|GetStaticMesh) _mesh))))